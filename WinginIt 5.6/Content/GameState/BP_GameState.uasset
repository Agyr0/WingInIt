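; Game state Blueprint that exposes the match's player list and filters it for spectating.
; GetCurrentPlayers returns the stored AllPlayers list and CurrentNumPlayers count, neither of which is updated in these graphs.
; GetSpectatablePlayers casts each player's pawn to BP_Chicken_FirstPerson and returns a unique list of those whose chicken is not dead.
; BeginPlay, Tick and the construction script hold no logic.
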(event `self.ReceiveBeginPlay`)

(fn `GetCurrentPlayers`
  (returns (AllPlayers :type "Array of /Game/GameState/BP_PlayerState Object Reference") (CurrentNumPlayers :type Integer))
  (return (`self.All Players`) (`self.Current Num Players`)))

(fn `GetSpectatablePlayers`
  (returns (Local_SpectatablePlayers :type "Array of /Game/GameState/BP_PlayerState Object Reference"))
  (locals (Local_Players :type "Array of /Game/GameState/BP_PlayerState Object Reference"))
  (for _array_element (`self.All Players`)
    (bind _asbp_chicken_first_person (cast `/Game/Player/BP_Chicken_FirstPerson` (`PlayerState.GetPawn` _array_element)))
    (if (not (`/Game/Player/BP_Chicken_FirstPerson.IsDead` _asbp_chicken_first_person))
      (`KismetArrayLibrary.Array_AddUnique` (`local.Local_Players`) _array_element)))
  (return (`local.Local_Players`)))

(fn `UserConstructionScript`)