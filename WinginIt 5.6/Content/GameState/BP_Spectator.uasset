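; BP_Spectator is a spectator pawn that orbits and looks at its attach parent, with key 1 repossessing the original player.
; Possession swaps the player input mapping for the spectator one.
; Move input drives RotatingMovement's rate, while zoom offsets the pawn within distance limits from the parent's "Spectator" socket and updates the orbit pivot.
; Tick locks rotation onto the parent; an interpolated distance-constraint function exists but is never called here.
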(event `self.ReceiveTick`
  (params (DeltaSeconds :type "Float (single-precision)"))
  ; Lock Rotation
  (`self.OGPlayer`
    (:`then`
      (`self.K2_SetActorRotation` (`KismetMathLibrary.FindLookAtRotation` (`self.K2_GetActorLocation`) (`self.K2_GetActorLocation` (`self.GetAttachParentActor`)))))
    (:`else`)))

(event `EnhancedInput|/Game/Input/Actions/Spectator/IA_SpectatorZoom`
  (params (ActionValue :type "Vector2D Structure") (ElapsedSeconds :type "Float (double-precision)") (TriggeredSeconds :type "Float (double-precision)") (InputAction :type "InputAction Object Reference" :default "/Game/Input/Actions/Spectator/IA_SpectatorZoom.IA_SpectatorZoom"))
  (:`Triggered`
    (set `self.DistanceToPlayer` (`KismetMathLibrary.Vector_Distance` (`SceneComponent.GetSocketLocation` (`Actor.RootComponent` (`self.GetAttachParentActor`)) "Spectator") (`self.K2_GetActorLocation`)))
    (if (or (and (< (`self.DistanceToPlayer`) (`self.MaxDistance`)) (< ActionValue_X 0.0)) (and (> (`self.DistanceToPlayer`) (`self.MinDistance`)) (> ActionValue_X 0.0)))
      (`self.K2_AddActorLocalOffset` (`KismetMathLibrary.MakeVector` (* ActionValue_X 10.0)))
      (set `RotatingMovementComponent.PivotTranslation` (`KismetMathLibrary.MakeVector` (`self.DistanceToPlayer`)) (`self.RotatingMovement`)))))

(event `EnhancedInput|/Game/Input/Actions/Spectator/IA_SpectatorMove`
  (params (ActionValue :type "Vector2D Structure") (ElapsedSeconds :type "Float (double-precision)") (TriggeredSeconds :type "Float (double-precision)") (InputAction :type "InputAction Object Reference" :default "/Game/Input/Actions/Spectator/IA_SpectatorMove.IA_SpectatorMove"))
  (:`Triggered`
    (if true
      (set `RotatingMovementComponent.RotationRate` (`KismetMathLibrary.MakeRotator` 0.0 (* ActionValue_Y 200.0) (* ActionValue_X 200.0)) (`self.RotatingMovement`))))
  (:`Completed`
    (set `RotatingMovementComponent.RotationRate` (`KismetMathLibrary.MakeRotator` 0.0) (`self.RotatingMovement`))))

(event `self.ReceivePossessed`
  (params (NewController :type "Controller Object Reference"))
  (bind _returnvalue (pcsubsystem `EnhancedInputLocalPlayerSubsystem` (`GameplayStatics.GetPlayerController` 0)))
  ; On Possessed
  (`/Engine/EditorBlueprintResources/StandardMacros.IsValid` _returnvalue
    (:`Is Valid`
      (message `EnhancedInputSubsystemInterface.AddMappingContext` _returnvalue "/Game/Input/IMC_Spectator.IMC_Spectator" 0 (struct))
      (`EnhancedInputSubsystemInterface.RemoveMappingContext` _returnvalue "/Game/Input/IMC_Player.IMC_Player" (struct)))))

(event `Key|One`
  (params (Key :type "Key Structure"))
  (:`Pressed`
    (`Controller.Possess` (`GameplayStatics.GetPlayerController` 0) (`self.OGPlayer`))))

(fn `ConstrainDistanceFromPlayer`
  (if (> (`KismetMathLibrary.Vector_Distance` (`self.K2_GetActorLocation`) (`self.K2_GetActorLocation` (`self.GetAttachParentActor`))) 1000.0)
    (`self.K2_SetActorLocation` (`KismetMathLibrary.VInterpTo` (`self.K2_GetActorLocation`) (+ (`self.K2_GetActorLocation` (`self.GetAttachParentActor`)) 1000.0) (`GameplayStatics.GetWorldDeltaSeconds`) 15.0))))

(fn `UserConstructionScript`)