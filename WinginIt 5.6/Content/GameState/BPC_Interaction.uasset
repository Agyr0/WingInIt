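; Interaction component that lets the player focus and use objects implementing BPI_Interactable.
; Each tick it line-traces from the player 0 pawn, drawing persistent debug, and sends FocusTarget with the hit component.
; The trace end is the forward vector times InteractionDistance, without adding the pawn location.
; IA_Interact reuses the last hit to call Interact, passing the pawn's owner as Interactor along with the hit component.
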(event `self.ReceiveTick`
  (params (DeltaSeconds :type "Float (single-precision)"))
  (bind _returnvalue (`GameplayStatics.GetPlayerPawn` 0))
  (bind _outhit (`KismetSystemLibrary.LineTraceSingle` :`Start` (`Actor.K2_GetActorLocation` _returnvalue) :`End` (* (`Actor.GetActorForwardVector` _returnvalue) (`self.Interaction Distance`)) :`TraceChannel` "TraceTypeQuery3" :`DrawDebugType` "Persistent"))
  (set `self.Out Hit` _outhit)
  (bind (_bblockinghit _binitialoverlap _time _distance _location _impactpoint _normal _impactnormal _physmat _hitactor _hitcomponent) (`GameplayStatics.BreakHitResult` _outhit))
  (bind _asbpi_interactable (cast `/Game/Player/BPI_Interactable` _hitactor))
  (`/Game/Player/BPI_Interactable.FocusTarget` _asbpi_interactable _hitcomponent))

(event `EnhancedInput|/Game/Input/Actions/Player/IA_Interact`
  (params (ActionValue :type Boolean) (ElapsedSeconds :type "Float (double-precision)") (TriggeredSeconds :type "Float (double-precision)") (InputAction :type "InputAction Object Reference" :default "/Game/Input/Actions/Player/IA_Interact.IA_Interact"))
  (bind (_out_hit_bblockinghit _out_hit_binitialoverlap _out_hit_time _out_hit_distance _out_hit_location _out_hit_impactpoint _out_hit_normal _out_hit_impactnormal _out_hit_physmat _out_hit_hitactor _out_hit_hitcomponent) (`GameplayStatics.BreakHitResult` (`self.Out Hit`)))
  (:`Triggered`
    (bind _asbpi_interactable (cast `/Game/Player/BPI_Interactable` _out_hit_hitactor))
    (`/Game/Player/BPI_Interactable.Interact` _asbpi_interactable (`Actor.GetOwner` (`GameplayStatics.GetPlayerPawn` 0)) _out_hit_hitcomponent)))