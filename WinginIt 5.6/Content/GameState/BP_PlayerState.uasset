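; Player state that shows a loading screen and assigns a net ID to the first-person chicken character when play begins.
; On BeginPlay it displays WB_LoadingScreen with a waiting-for-players message, then copies its unique ID into MyNetID on player 0's character.
; It uses AutomationWaitForLoading as the wait before removing the screen, which stays up if the character cast fails.
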(event `self.ReceiveBeginPlay`
  ; Create Loading Screen
  (bind _returnvalue (`|CreateWidget` "/Game/GameState/UI/WB_LoadingScreen.WB_LoadingScreen_C" null "Waiting for players to join"))
  (bind _output_get (set `self.LoadingScreen` _returnvalue))
  (`UserWidget.AddToViewport` _output_get 0)
  ; Assign Net ID
  (bind _asbp_chicken_first_person (cast `/Game/Player/BP_Chicken_FirstPerson` (`GameplayStatics.GetPlayerCharacter` 0)))
  (set `/Game/Player/BP_Chicken_FirstPerson.MyNetID` (`self.BP_GetUniqueId`) _asbp_chicken_first_person)
  ; Close Loading Screen
  (`AutomationBlueprintFunctionLibrary.AutomationWaitForLoading` (make `AutomationWaitForLoadingOptions` true))
  (`Widget.RemoveFromParent` (`self.LoadingScreen`)))

(fn `UserConstructionScript`)