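; BP_Campfire is a campfire actor with six child-actor eggs that signal when players have died.
; On BeginPlay it caches the game mode and state and binds to BP_GameState's OnPlayerDied event, which passes through server and multicast ReadyHatch events.
; SetEggReadyToHatch matches the dead player's ID in AllPlayers and loops the shake animation on the egg at that index.
; Interact and FocusTarget are placeholders.
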(event `self.ReceiveBeginPlay`
  (set `self.EggSpawns` (`|MakeArray` (`self.BP_Egg`) (`self.BP_Egg1`) (`self.BP_Egg2`) (`self.BP_Egg3`) (`self.BP_Egg4`) (`self.BP_Egg5`)))
  (bind _asbp_first_person_game_mode (cast `/Game/GameState/BP_FirstPersonGameMode` (`GameplayStatics.GetGameMode`))
    (:`then`
      (set `self.As BP First Person Game Mode` _asbp_first_person_game_mode))
    (:`CastFailed`
      _))
  (bind _asbp_game_state (cast `/Game/GameState/BP_GameState` (`GameplayStatics.GetGameState`)))
  (bind _output_get (set `self.As BP Game State` _asbp_game_state))
  (add `/Game/GameState/BP_GameState.OnPlayerDied` _output_get (delegate `ReadyHatch`)))

(event `ReadyHatch`
  (params (DeadPlayer :type "/Game/GameState/BP_PlayerState Object Reference"))
  (`self.ServerReadyHatch` DeadPlayer))

(event `ServerReadyHatch`
  (params (DeadPlayer :type "/Game/GameState/BP_PlayerState Object Reference"))
  (`self.MulticastReadyHatch` DeadPlayer))

(event `MulticastReadyHatch`
  (params (DeadPlayer :type "/Game/GameState/BP_PlayerState Object Reference"))
  (`self.SetEggReadyToHatch` DeadPlayer))

(event `/Game/Player/BPI_Interactable.Interact`
  (params (Interactor :type "Object Object Reference") (ComponentHit :type "SceneComponent Object Reference"))
  (`KismetSystemLibrary.PrintString` "Hello"))

(fn `FocusTarget`
  (params (ComponentHit :type "SceneComponent Object Reference"))
  (returns (Message :type Text))
  (return ""))

(fn `OnRep_EggSpawns`)

(fn `SetEggReadyToHatch`
  (params (DeadPlayer :type "/Game/GameState/BP_PlayerState Object Reference"))
  (`self.ForceNetUpdate`)
  (bind _as_bp_game_state (`self.As BP Game State`)
    (:`then`
      (for (_array_element _array_index) (`/Game/GameState/BP_GameState.All Players` _as_bp_game_state)
        (if (== (`PlayerState.PlayerId` _array_element) (`PlayerState.PlayerId` DeadPlayer))
          (bind _asbp_egg (cast `/Game/GameState/BP_Egg` (`ChildActorComponent.ChildActor` (`|GetArrayItem` (`self.EggSpawns`) _array_index))))
          (`SkeletalMeshComponent.PlayAnimation` (`/Game/GameState/BP_Egg.Egg` _asbp_egg) (`self.EggShake`) true))))
    (:`else`)))

(fn `UserConstructionScript`)