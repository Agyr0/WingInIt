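; BP_Egg is an egg actor that drops itself onto the surface below it when play begins.
; BeginPlay traces 100 units down from the Egg component on Visibility and moves the actor to the impact point without checking for a hit.
; Interact is empty and FocusTarget returns an empty string.
; Disconnected, never-run logic would spawn a player through BP_FirstPersonGameMode and play a break effect while hiding the egg.
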(event `self.ReceiveBeginPlay`
  (bind _returnvalue (`SceneComponent.K2_GetComponentLocation` (`self.Egg`)))
  (bind _outhit (`KismetSystemLibrary.LineTraceSingle` _returnvalue (`KismetMathLibrary.MakeVector` (.x _returnvalue) (.y _returnvalue) (- (.z _returnvalue) 100.0)) "TraceTypeQuery1"))
  (`self.K2_SetActorLocation` (`.ImpactPoint` (`GameplayStatics.BreakHitResult` _outhit))))

(event `/Game/Player/BPI_Interactable.Interact`
  (params (Interactor :type "Object Object Reference") (ComponentHit :type "SceneComponent Object Reference")))

(fn `FocusTarget`
  (params (ComponentHit :type "SceneComponent Object Reference"))
  (returns (Message :type Text))
  (return ""))

(fn `UserConstructionScript`)