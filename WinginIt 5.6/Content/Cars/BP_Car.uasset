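; BP_Car is a hazard car that repeatedly drives from a start point to an end point and kills chicken players it hits.
; After a random delay of up to two seconds, a multicast-named event plays a timeline that eases the mesh toward the end point with VInterpTo.
; On finish, the mesh teleports back to the start and the cycle repeats.
; Box overlap with BP_Chicken_FirstPerson calls its ServerDeath and fires a radial impulse.
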(event `self.ReceiveBeginPlay`
  (`AutomationBlueprintFunctionLibrary.AutomationWaitForLoading` (make `AutomationWaitForLoadingOptions` true))
  (`self.DriveCarServer`))

(event `DriveCarServer`
  (`KismetSystemLibrary.Delay` (`KismetMathLibrary.RandomFloatInRange` 0.0 2.0))
  (`self.DriveCarMulticast`))

(event `DriveCarMulticast`
  (`Timeline|MoveCar` :!via `PlayFromStart`
    (:`Update`
      (`SceneComponent.K2_SetWorldLocation` (`self.StaticMesh`) (`KismetMathLibrary.VInterpTo` (`SceneComponent.K2_GetComponentLocation` (`self.StaticMesh`)) (`SceneComponent.K2_GetComponentLocation` (`self.EndPos`)) (`GameplayStatics.GetWorldDeltaSeconds`) 1.0) false false))
    (:`Finished`
      (`SceneComponent.K2_SetWorldLocation` (`self.StaticMesh`) (`SceneComponent.K2_GetComponentLocation` (`self.StartPos`)) false false)
      (`self.DriveCarServer`))))

(event `self.Box.OnComponentBeginOverlap`
  (params (OverlappedComponent :type "PrimitiveComponent Object Reference") (OtherActor :type "Actor Object Reference") (OtherComp :type "PrimitiveComponent Object Reference") (OtherBodyIndex :type Integer) (bFromSweep :type Boolean) (SweepResult :type "HitResult Structure (by ref)"))
  (bind _asbp_chicken_first_person (cast `/Game/Player/BP_Chicken_FirstPerson` OtherActor))
  (`/Game/Player/BP_Chicken_FirstPerson.ServerDeath` _asbp_chicken_first_person)
  (`self.ServerImpulse`))

(event `ServerImpulse`
  (`RadialForceComponent.FireImpulse` (`self.RadialForce`) :!label _label))

(event `MulticastImpulse`
  (goto _label))

(fn `UserConstructionScript`)